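; Inventory Blueprint that holds items in a fixed number of slots, each storing an item class and amount.
; Helper functions check slots, read item class defaults, and search for empty slots or partial stacks of a class.
; AddItem writes non-stackable items one per slot by calling itself recursively, while its stackable branch only runs the stack search.
; As written, the empty-slot search never sets its success flag, and the stack search returns an amount as the index.
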(event `self.ReceiveBeginPlay`
  (`KismetArrayLibrary.Array_Resize` (`self.Slots`) (`self.amountofSlots`)))

(fn `AddItem`
  (params (itemclass :type "/Game/Inventory_system/Blueprints/itemClasses/mastreitem_BP Class Reference") (Amount :type Integer))
  (returns (`Success?` :type Boolean))
  (locals (LocalClass :type "/Game/Inventory_system/Blueprints/itemClasses/mastreitem_BP Class Reference") (LocalAmount :type Integer) (FoundIndex :type Integer))
  (set `local.LocalClass` itemclass)
  (set `local.LocalAmount` Amount)
  (if (`.canBeStacked?_19_4F73F76E4D0979E4B8AA78AAC383EC0A` (break `/Game/Inventory_system/Blueprints/Structures/s_itemInfo_BP` (defaults `/Game/Inventory_system/Blueprints/inventory_BP` itemclass)))
    (`self.SearchFreeStack` (`local.LocalClass`))
    (else
      (bind (_success_ _index) (`self.SearchEmptySlots`))
      (if _success_
        (bind _output_get (set `local.FoundIndex` _index))
        (`KismetArrayLibrary.Array_Set` (`self.Slots`) _output_get (make `/Game/Inventory_system/Blueprints/Structures/s_inventory_slots` (`local.LocalClass`) 1))
        (if (>= (`local.LocalAmount`) 1)
          (`self.AddItem` (`local.LocalClass`) (- (`local.LocalAmount`) 1))
          (return true)
          (else
            (return false)))
        (else
          (return false))))))

(fn `GetitemInfoAtIndex`
  (params (index :type Integer))
  (returns (`EmptySlot?` :type Boolean) (itemInfo :type "/Game/Inventory_system/Blueprints/Structures/s_itemInfo_BP Structure") (Amount :type Integer))
  (bind (_itemclass _amount) (break `/Game/Inventory_system/Blueprints/Structures/s_inventory_slots` (`|GetArrayItem` (`self.Slots`) index)))
  (if (`KismetSystemLibrary.IsValidClass` _itemclass)
    (return false (defaults `/Game/Inventory_system/Blueprints/inventory_BP` _itemclass) _amount)
    (else
      (return true (struct) 0))))

(fn `isSlotEmpty`
  (params (index :type Integer))
  (returns (`Empty?` :type Boolean))
  (return (not (`KismetSystemLibrary.IsValidClass` (`.itemClass_2_EC935844482CCD8CDCDD988BF991E24F` (break `/Game/Inventory_system/Blueprints/Structures/s_inventory_slots` (`|GetArrayItem` (`self.Slots`) index)))))))

(fn `SearchEmptySlots`
  (returns (`Success?` :type Boolean) (index :type Integer))
  (locals (LocalBool :type Boolean) (localIndex :type Integer))
  (for (_array_element _array_index) (`self.Slots`)
    (if (not (`KismetSystemLibrary.IsValidClass` (`.itemClass_2_EC935844482CCD8CDCDD988BF991E24F` (break `/Game/Inventory_system/Blueprints/Structures/s_inventory_slots` _array_element))))
      (set `local.localIndex` _array_index)
      (break)))
  (return (`local.LocalBool`) (`local.localIndex`)))

(fn `SearchFreeStack`
  (params (itemClass :type "/Game/Inventory_system/Blueprints/itemClasses/mastreitem_BP Class Reference"))
  (returns (`Sucess?` :type Boolean) (index :type Integer))
  (locals (LocalBool :type Boolean) (localIndex :type Integer))
  (for _array_element (`self.Slots`)
    (bind (_itemclass _amount) (break `/Game/Inventory_system/Blueprints/Structures/s_inventory_slots` _array_element))
    (if (`KismetSystemLibrary.IsValidClass` _itemclass)
      (if (and (== _itemclass itemClass) (< _amount (`self.maxStackSize`)))
        (set `local.LocalBool` true)
        (set `local.localIndex` _amount)
        (break))))
  (return (`local.LocalBool`) (`local.localIndex`)))

(fn `UserConstructionScript`)