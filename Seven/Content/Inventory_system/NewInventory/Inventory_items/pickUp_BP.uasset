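; World pickup actor that adds its item to the player's inventory when Equip is pressed inside its overlap sphere.
; Overlap events toggle CanPickup on pickup and player, and both enable input, leaving the flag to gate pickup.
; Consumables merge counts with same-named inventory entries; other items are appended with a new index.
; Either path updates the MyInventory widget directly and destroys the actor.
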(event `self.ReceiveBeginPlay`
  ;[1 1 1] Begin Play
  (bind _asplayer_bp (cast `/Game/Blueprints/Player/Player_BP` (`GameplayStatics.GetPlayerCharacter` 0)))
  (set `self.Player` _asplayer_bp))

(event `InputAction|Equip`
  (params (Key :type "Key Structure"))
  (bind (_itemindex _itemname _itemcount _icon _description _weight _isconsumable_ _usage _weaponsocketname _weaponactor) (break `/Game/Blueprints/Player/S_itemDetails` (`self.itemDetail`)))
  (bind _inventoryitems (`/Game/Blueprints/Player/Player_BP.InventoryItems` (`self.Player`)))
  ;[1 1 1] can pick pickUps if certain key is pressed
  (:`Pressed`
    (if (`self.canPickup`)
      (bind _similaritempresent_ (`self.isSimilarItemPresent`))
      (if (not _similaritempresent_)
        (bind _output_get (set `self.itemDetail` (make `/Game/Blueprints/Player/S_itemDetails` (`KismetArrayLibrary.Array_Length` _inventoryitems) _itemname _itemcount _icon _description _weight _isconsumable_ _usage _weaponsocketname _weaponactor)))
        (bind _returnvalue (`KismetArrayLibrary.Array_Add` _inventoryitems _output_get))
        (bind _foundwidgets (`WidgetBlueprintLibrary.GetAllWidgetsOfClass` "/Game/Inventory_system/NewInventory/Inventory_widgets/myInventory.myInventory_C"))
        (`/Game/Inventory_system/NewInventory/Inventory_widgets/myInventory.addItems` (`|GetArrayItem` _foundwidgets) _returnvalue)
        (`self.K2_DestroyActor`)))))

(event `self.Sphere.OnComponentBeginOverlap`
  (params (OverlappedComponent :type "PrimitiveComponent Object Reference") (OtherActor :type "Actor Object Reference") (OtherComp :type "PrimitiveComponent Object Reference") (OtherBodyIndex :type Integer) (bFromSweep :type Boolean) (SweepResult :type "HitResult Structure (by ref)"))
  (bind _player (`self.Player`))
  (if (== OtherActor _player)
    (set `/Game/Blueprints/Player/Player_BP.canPickUp` true _player)
    (set `self.canPickup` true)
    (`self.EnableInput` (`GameplayStatics.GetPlayerController` 0))))

(event `self.Sphere.OnComponentEndOverlap`
  (params (OverlappedComponent :type "PrimitiveComponent Object Reference") (OtherActor :type "Actor Object Reference") (OtherComp :type "PrimitiveComponent Object Reference") (OtherBodyIndex :type Integer))
  (bind _player (`self.Player`))
  (if (== OtherActor _player)
    (set `/Game/Blueprints/Player/Player_BP.canPickUp` false _player)
    (set `self.canPickup` false)
    (`self.EnableInput` (`GameplayStatics.GetPlayerController` 0))))

(fn `isSimilarItemPresent`
  (returns (`SimilarItemPresent?` :type Boolean))
  (locals (`SimilarItem?` :type Boolean))
  (bind (_itemdetail_itemindex _itemdetail_itemname _itemdetail_itemcount _itemdetail_icon _itemdetail_description _itemdetail_weight _itemdetail_isconsumable_) (break `/Game/Blueprints/Player/S_itemDetails` (`self.itemDetail`)))
  (for (_array_element _array_index) (`/Game/Blueprints/Player/Player_BP.InventoryItems` (`self.Player`))
    (if _itemdetail_isconsumable_
      (if (== _itemdetail_itemname (`.ItemName_2_C5DF740E435E63E333DE0593520D5347` (break `/Game/Blueprints/Player/S_itemDetails` _array_element)))
        (bind _returnvalue (+ (`.itemCount_35_18E5D2FC4B4222468AFB5383114CA6ED` (break `/Game/Blueprints/Player/S_itemDetails` _array_element)) _itemdetail_itemcount))
        (`KismetArrayLibrary.Array_Set` (`/Game/Blueprints/Player/Player_BP.InventoryItems` (`self.Player`)) _array_index (make `/Game/Blueprints/Player/S_itemDetails` (break `/Game/Blueprints/Player/S_itemDetails` _array_element) (`.ItemName_2_C5DF740E435E63E333DE0593520D5347` (break `/Game/Blueprints/Player/S_itemDetails` _array_element)) _returnvalue (`.Icon_5_2FB7132747B6638DA05CF2B25F0B7715` (break `/Game/Blueprints/Player/S_itemDetails` _array_element)) (`.Description_11_BC4398BB45F9AE4367460B93869D0D5C` (break `/Game/Blueprints/Player/S_itemDetails` _array_element)) (`.Weight_8_1617027A4949C5E47F82B5949121CA19` (break `/Game/Blueprints/Player/S_itemDetails` _array_element)) (`.IsConsumable?_14_EC08519F445304A8D16B909EA35E9E0E` (break `/Game/Blueprints/Player/S_itemDetails` _array_element)) (`.Usage_19_C87C3C5744444D3B9AF734A6009CDD3F` (break `/Game/Blueprints/Player/S_itemDetails` _array_element)) (`.WeaponSocketName_25_6063081B421F17C9A0D78DA3AAD4E54D` (break `/Game/Blueprints/Player/S_itemDetails` _array_element)) (`.WeaponActor_29_2BED244F4C30F3BB25897A857F4D5FFB` (break `/Game/Blueprints/Player/S_itemDetails` _array_element))))
        (set `local.SimilarItem?` true)
        (`KismetSystemLibrary.PrintString` (`KismetStringLibrary.Conv_IntToString` _returnvalue))
        (bind _foundwidgets (`WidgetBlueprintLibrary.GetAllWidgetsOfClass` "/Game/Inventory_system/NewInventory/Inventory_widgets/myInventory.myInventory_C"))
        (bind _output (`|GetArrayItem` _foundwidgets))
        (`/Game/Inventory_system/NewInventory/Inventory_widgets/myInventory.removeItems` _output _array_index)
        (`/Game/Inventory_system/NewInventory/Inventory_widgets/myInventory.addItems` _output _array_index)
        (`self.K2_DestroyActor`)
        (break)
        (else
          (set `local.SimilarItem?` false)))))
  (return (`local.SimilarItem?`)))

(fn `UserConstructionScript`)