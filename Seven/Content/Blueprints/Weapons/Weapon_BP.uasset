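; Weapon actor that the player can pick up into the inventory and that deals hit damage between the player and AI enemies.
; Overlapping the equip sphere enables input, and Equip adds its item details to the inventory, refreshes the widget and destroys the actor.
; Weapon overlaps call ApplyWeaponDamage on the victim, gated by the attacker's CanApplyDamage and DoOnce nodes.
; Tick toggles physics and pickup radius according to whether the weapon is possessed.
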(event `InputAction|Equip`
  (params (Key :type "Key Structure"))
  ;[1 1 1] Equip button pressed
  (:`Pressed`
    (if (`self.canPickUp`)
      (if (not (`self.ispossessed`))
        (`self.addToInventory`)))))

(event `self.EquipBound.OnComponentBeginOverlap`
  (params (OverlappedComponent :type "PrimitiveComponent Object Reference") (OtherActor :type "Actor Object Reference") (OtherComp :type "PrimitiveComponent Object Reference") (OtherBodyIndex :type Integer) (bFromSweep :type Boolean) (SweepResult :type "HitResult Structure (by ref)"))
  ;[1 1 1] Can Equip Weapon
  (if (== OtherActor (`self.PlayerCharcter`))
    (set `self.canPickUp` true)
    (`self.EnableInput` (`GameplayStatics.GetPlayerController` 0))))

(event `self.EquipBound.OnComponentEndOverlap`
  (params (OverlappedComponent :type "PrimitiveComponent Object Reference") (OtherActor :type "Actor Object Reference") (OtherComp :type "PrimitiveComponent Object Reference") (OtherBodyIndex :type Integer))
  ;[1 1 1] Cant equip Weapon
  (if (== OtherActor (`self.PlayerCharcter`))
    (set `self.canPickUp` false)))

(event `self.weapon.OnComponentBeginOverlap`
  (params (OverlappedComponent :type "PrimitiveComponent Object Reference") (OtherActor :type "Actor Object Reference") (OtherComp :type "PrimitiveComponent Object Reference") (OtherBodyIndex :type Integer) (bFromSweep :type Boolean) (SweepResult :type "HitResult Structure (by ref)"))
  (bind _playercharcter (`self.PlayerCharcter`))
  (bind _playercharcter_2 (`self.PlayerCharcter`))
  (set `self.OverlappedActor` OtherActor)
  (set `self.thisWeapon` self)
  (if (== (`self.OverlappedActor`) (`self.PlayerCharcter`))
    ;[1 1 1] player is taking damage
    (bind _outactors (`GameplayStatics.GetAllActorsOfClass` "/Game/Blueprints/AI/AI_BP.AI_BP_C"))
    (for _array_element _outactors :!label _label
      (if (== (`HumanCharacter.MyWeapon` _array_element) (`self.thisWeapon`))
        (`self.Break`)
        (bind _output_get (set `self.AICharacter` _array_element))
        (if (`HumanCharacter.canApplyDamage` _output_get)
          (`/Engine/EditorBlueprintResources/StandardMacros.DoOnce` false :!label _label_2
            (:`Completed`
              (`HumanCharacter.applyWeaponDamage` _playercharcter_2 (`self.thisWeapon`) (`self.AICharacter`) _playercharcter_2)))
          (else
            (goto _label_2 :!via `Reset`)))))
    (else
      ;[1 1 1] Enemy is Taking Damage
      (`/Engine/EditorBlueprintResources/StandardMacros.IsValid` _playercharcter
        (:`Is Valid`
          (if (`HumanCharacter.canApplyDamage` _playercharcter)
            (bind _asai_bp (cast `/Game/Blueprints/AI/AI_BP` (`self.OverlappedActor`)))
            (`/Engine/EditorBlueprintResources/StandardMacros.DoOnce` false :!label _label_3
              (:`Completed`
                (`HumanCharacter.applyWeaponDamage` _asai_bp (`self.thisWeapon`) (`self.PlayerCharcter`) _asai_bp)))
            (else
              (goto _label_3 :!via `Reset`))))))))

(event `Break`
  ;[1 1 1] player is taking damage
  (goto _label :!via `Break`))

(event `self.ReceiveBeginPlay`
  ;[1 1 1] Begin Play
  (bind _asplayer_bp (cast `/Game/Blueprints/Player/Player_BP` (`GameplayStatics.GetPlayerCharacter` 0)))
  (set `self.PlayerCharcter` _asplayer_bp))

(event `self.ReceiveTick`
  (params (DeltaSeconds :type "Float (single-precision)"))
  (if (`self.ispossessed`)
    (`PrimitiveComponent.SetSimulatePhysics` (`self.weapon`) false)
    (`SphereComponent.SetSphereRadius` (`self.EquipBound`) 0.0 false)
    (else
      (`PrimitiveComponent.SetSimulatePhysics` (`self.weapon`) true)
      (`SphereComponent.SetSphereRadius` (`self.EquipBound`) 150.0 true))))

(fn `addToInventory`
  (bind _returnvalue (`KismetArrayLibrary.Array_Add` (`/Game/Blueprints/Player/Player_BP.InventoryItems` (`self.PlayerCharcter`)) (`self.item_details`)))
  (bind _foundwidgets (`WidgetBlueprintLibrary.GetAllWidgetsOfClass` "/Game/Inventory_system/NewInventory/Inventory_widgets/myInventory.myInventory_C"))
  (`/Game/Inventory_system/NewInventory/Inventory_widgets/myInventory.addItems` (`|GetArrayItem` _foundwidgets) _returnvalue)
  (`self.K2_DestroyActor`))

(fn `UserConstructionScript`
  (bind (_item_details_itemname _item_details_icon _item_details_description _item_details_weight _item_details_isconsumable_ _item_details_usage) (break `/Game/Blueprints/Player/S_itemDetails` (`self.item_details`)))
  (set `self.weaponDamage` _item_details_usage))