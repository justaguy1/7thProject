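; Player character Blueprint that creates the HUD, shortcut, inventory, skill and pause widgets and handles movement speed, menus and equipment input.
; Target lock-on uses a timeline to interpolate control yaw toward the enemy while damping look input.
; Right-hand slots cycle to spawn and socket-attach weapons, which set attack montage and type; Tab drops them.
; Left-hand slots cycle healing items, syncing counts to inventory; overlap damage logic is disconnected.
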(event OnComponentBeginOverlap(CapsuleComponent)
  (params (OverlappedComponent :type Primitive%20Component%20Object%20Reference) (OtherActor :type Actor%20Object%20Reference) (OtherComp :type Primitive%20Component%20Object%20Reference) (OtherBodyIndex :type Integer) (bFromSweep :type Boolean) (SweepResult :type Hit%20Result%20Structure%20%28by%20ref%29))
  ;[1 1 1] get damage from enemy
)

(event Custom|Breakloop
  ;[1 1 1] get damage from enemy
  (Utilities|Array|ForEachLoopwithBreak (stale _outactors)) ; enters at Break
)

(event EventBeginPlay
  ;[1 1 1] begin play
  (CallFunction|SetMontages)
  (bind _returnvalue (UserInterface|CreateWidget "/Game/Blueprints/Huds/player_hud.player_hud_C"))
  (UserInterface|Viewport|AddtoViewport _returnvalue 0)
  (CallFunction|SetInventoryWidget)
  (CallFunction|SetSkillWidget)
  (bind _returnvalue_2 (UserInterface|CreateWidget "/Game/Inventory_system/NewInventory/Inventory_widgets/Shortcut_Widget.Shortcut_Widget_C"))
  (bind _output_get (Variables|Default|SetShortcutWidgetInstance _returnvalue_2))
  (UserInterface|Viewport|AddtoViewport _output_get 0)
  (bind _returnvalue_3 (UserInterface|CreateWidget "/Game/Inventory_system/pauseMenu.pauseMenu_C"))
  (bind _output_get_2 (Variables|Default|SetPausewidgetInstance _returnvalue_3))
  (UserInterface|Viewport|AddtoViewport _output_get_2 0))

(event EventTick
  (params (DeltaSeconds :type Float%20%28single-precision%29)))

(event Input|ActionEvents|InputActionTargetEnemy
  (params (Key :type Key%20Structure))
  (bind _enemy (Variables|Default|Getenemy))
  ;[1 1 1] Target system input
  (:Pressed
    (Class|PlayerHumanCharacter|TargetEnemy)
    (Utilities|IsValid _enemy
      (:Is%20Valid
        (if (Variables|/Script/Seven.AIHumanCharacter|Gettargeted _enemy)
          (Variables|Default|SettargetLockOn true)
          (Timeline|Timeline_0 Play
            (:Update
              (CallFunction|EnemyTargetSystem)))
          (else
            (Variables|Default|SettargetLockOn false)
            (Timeline|Timeline_0 Stop)))))))

(event Input|ActionEvents|InputActionInventory
  (params (Key :type Key%20Structure))
  ;[1 1 1] Open And Close Inventory
  (:Pressed
    (bind _output_get (Variables|Default|SetopenInventory (not (Variables|Default|GetopenInventory))))
    (if _output_get
      (Widget|SetVisibility (Variables|Default|GetInventoryInstance) "Visible")
      (Variables|/Script/Engine.PlayerController|SetbShowMouseCursor (Game|GetPlayerController 0) true)
      (else
        (Widget|SetVisibility (Variables|Default|GetInventoryInstance) "Hidden")
        (Variables|/Script/Engine.PlayerController|SetbShowMouseCursor (Game|GetPlayerController 0) false)))))

(event Input|AxisEvents|InputAxisTurn
  (params (AxisValue :type Float%20%28single-precision%29))
  ;[1 1 1] clamped targeting system
  (Pawn|Input|AddControllerYawInput (* (Math|Float|SelectFloat 0.2 1.0 (Variables|Default|GettargetLockOn)) AxisValue)))

(event Input|AxisEvents|InputAxisLookUp
  (params (AxisValue :type Float%20%28single-precision%29))
  ;[1 1 1] clamped targeting system
  (Pawn|Input|AddControllerPitchInput (* (Math|Float|SelectFloat 0.2 1.0 (Variables|Default|GettargetLockOn)) AxisValue)))

(event Input|KeyboardEvents|LeftCtrl
  (params (Key :type Key%20Structure))
  ;[1 1 1] walk / run
  (:Pressed
    (Variables|/Script/Engine.CharacterMovementComponent|SetMaxWalkSpeed (Variables|Character|GetCharacterMovement) 6e+02))
  (:Released
    (Variables|/Script/Engine.CharacterMovementComponent|SetMaxWalkSpeed (Variables|Character|GetCharacterMovement) 3e+02)))

(event Input|KeyboardEvents|F
  (params (Key :type Key%20Structure))
  (:Pressed
    (Utilities|FlowControl|DoOnce false :!label _label
      (:Completed
        (CallFunction|CheckWhichItemtoUse))))
  (:Released
    (goto _label Reset)))

(event Input|KeyboardEvents|K
  (params (Key :type Key%20Structure))
  (:Pressed
    (bind _output_get (Variables|Default|SetopenInventory (not (Variables|Default|GetopenInventory))))
    (if _output_get
      (Widget|SetVisibility (Variables|Default|GetSkillWidgetInstance) "Visible")
      (else
        (Widget|SetVisibility (Variables|Default|GetSkillWidgetInstance) "Hidden")))))

(event Input|KeyboardEvents|Left
  (params (Key :type Key%20Structure))
  (:Pressed
    (Utilities|FlowControl|DoOnce false :!label _label
      (:Completed
        (CallFunction|SwitchItems))))
  (:Released
    (goto _label Reset)))

(event Input|KeyboardEvents|Right
  (params (Key :type Key%20Structure))
  (:Pressed
    (Utilities|FlowControl|DoOnce false :!label _label
      (:Completed
        (CallFunction|SwitchWeapons))))
  (:Released
    (goto _label Reset)))

(event Input|KeyboardEvents|P
  (params (Key :type Key%20Structure))
  ;[1 1 1] Pause menu
  (:Pressed
    (bind _output_get (Variables|Default|Setpause (not (Variables|Default|Getpause))))
    (if _output_get
      (Widget|SetVisibility (Variables|Default|GetPausewidgetInstance) "Visible")
      (Variables|/Script/Engine.PlayerController|SetbShowMouseCursor (Game|GetPlayerController 0) true)
      (Game|SetGamePaused (Variables|Default|Getpause)))))

(event Input|KeyboardEvents|Tab
  (params (Key :type Key%20Structure))
  (bind _righthanditems (Variables|Default|GetRightHandItems))
  ;[1 1 1] Un equip Weapon
  (:Pressed
    (Variables|Default|SetcanEquip false)
    (Utilities|IsValid (Variables|Default|GetMyWeapon)
      (:Is%20Valid
        (bind _asweapon_bp (Utilities|Casting|CastToWeapon_BP (Variables|Default|GetMyWeapon)))
        (Variables|/Script/Seven.Weapon|Setispossessed _asweapon_bp false)
        (Transformation|DetachFromActor _asweapon_bp "KeepWorld" "KeepWorld" "KeepWorld")
        (Components|Sphere|SetSphereRadius (Variables|/Game/Blueprints/Weapons/Weapon_BP.Weapon_BP_C|GetEquipBound _asweapon_bp) 1e+02 true)
        (Variables|Default|SetIsWeaponEquipped false)
        (CallFunction|RemoveIconwhenUnequipped (Variables|Default|GetweaponToEquip%20Index))
        (Utilities|Array|RemoveIndex (Variables|Default|GetInventoryItems) (.itemIndex (Utilities|Struct|BreakS_itemDetails (Variables|/Game/Blueprints/Weapons/Weapon_BP.Weapon_BP_C|Getitem_details (.AsWeapon%20BP (Utilities|Casting|CastToWeapon_BP (Variables|Default|GetMyWeapon)))))))
        (Variables|Default|SetMyWeapon 0)
        (bind _returnvalue (Utilities|Array|Add (Variables|Default|GetRightHandItems) (Variables|Default|GetNullValueForiteam)))
        (Utilities|Array|Swap _righthanditems (Variables|Default|GetweaponToEquip%20Index) _returnvalue)
        (Utilities|Array|RemoveIndex _righthanditems 3)
        (CallFunction|SwitchWeapons)))))

(fn ConstructionScript
  (Variables|Default|SetWeaponType "NewEnumerator1"))

(fn SetMontages
  (Variables|Default|SetanimInstance (Components|SkeletalMesh|GetAnimInstance (Variables|Character|GetMesh)))
  (Variables|Default|SetattackMontage (Utilities|Array|MakeArray "/Game/Models/VampireAnimations/slash_01.slash_01" "/Game/Models/VampireAnimations/Attack_torch.Attack_torch" "/Game/Models/VampireAnimations/slash_02.slash_02"))
  (Variables|Default|SetreactMontage (Utilities|Array|MakeArray "/Game/Models/VampireAnimations/react_left.react_left" "/Game/Models/VampireAnimations/react_right.react_right")))

(fn EnemyTargetSystem
  (bind _returnvalue (Pawn|GetController))
  (bind _enemy (Variables|Default|Getenemy))
  (bind _returnvalue_2 (Pawn|GetControlRotation _returnvalue :!class /Script/Engine.Controller))
  (bind (_roll _pitch) (Math|Rotator|BreakRotator _returnvalue_2))
  (Utilities|IsValid _enemy
    (:Is%20Valid
      (Pawn|SetControlRotation (Pawn|GetController) (Math|Rotator|MakeRotator _roll _pitch (.Yaw (Math|Rotator|BreakRotator (Math|Interpolation|RInterpTo _returnvalue_2 (Math|Rotator|FindLookatRotation (Transformation|GetWorldLocation (Variables|Default|GetFollowCamera)) (Transformation|GetActorLocation _enemy)) (Utilities|Time|GetWorldDeltaSeconds) 7.0))))))))

(fn SetInventoryWidget
  (bind _returnvalue (UserInterface|CreateWidget "/Game/Inventory_system/NewInventory/Inventory_widgets/myInventory.myInventory_C"))
  (bind _output_get (Variables|Default|SetInventoryInstance _returnvalue))
  (UserInterface|Viewport|AddtoViewport _output_get 0)
  (Widget|SetVisibility (Variables|Default|GetInventoryInstance) "Hidden"))

(fn AttachWeapon
  (bind _myweapon (Variables|Default|GetMyWeapon))
  (Utilities|IsValid _myweapon
    (:Is%20Valid
      (bind _asweapon_bp (Utilities|Casting|CastToWeapon_BP _myweapon))
      (Transformation|AttachComponentToComponent _asweapon_bp (Variables|Character|GetMesh) (.WeaponSocketName (Utilities|Struct|BreakS_itemDetails (Variables|/Game/Blueprints/Weapons/Weapon_BP.Weapon_BP_C|Getitem_details _asweapon_bp))) "SnapToTarget" "SnapToTarget" "SnapToTarget" true)
      (Variables|/Script/Seven.Weapon|Setispossessed _asweapon_bp true)
      (Components|Sphere|SetSphereRadius (Variables|/Game/Blueprints/Weapons/Weapon_BP.Weapon_BP_C|GetEquipBound _asweapon_bp) 0.0 false)
      (Variables|Default|SetIsWeaponEquipped true)
      (Utilities|IsValid _asweapon_bp
        (:Is%20Valid
          (Variables|Default|SetattackMontage (Utilities|Array|MakeArray (Utilities|Array|Get(acopy) (Variables|/Game/Blueprints/Weapons/Weapon_BP.Weapon_BP_C|GetattackMontage _asweapon_bp))))
          (Variables|Default|SetWeaponType (Variables|/Game/Blueprints/Weapons/Weapon_BP.Weapon_BP_C|GetSwordType _asweapon_bp)))))))

(fn SetSkillWidget
  (bind _returnvalue (UserInterface|CreateWidget "/Game/Blueprints/Huds/SkillPointHud.SkillPointHud_C"))
  (bind _output_get (Variables|Default|SetSkillWidgetInstance _returnvalue))
  (UserInterface|Viewport|AddtoViewport _output_get 0)
  (Widget|SetVisibility _output_get "Hidden"))

(fn SpawnWeapon
  (Utilities|IsValid (Variables|Default|GetMyWeapon)
    (:Is%20Valid
      (Actor|DestroyActor (Variables|Default|GetMyWeapon)))
    (:Is%20Not%20Valid
      _))
  (Variables|Default|SetMyWeapon 0)
  (Variables|Default|SetIsWeaponEquipped false)
  (bind _returnvalue (Game|SpawnActorfromClass (.WeaponActor (Utilities|Struct|BreakS_itemDetails (Utilities|Array|Get(acopy) (Variables|Default|GetRightHandItems) (Variables|Default|GetweaponToEquip%20Index)))) (Transformation|GetWorldTransform (Variables|Character|GetMesh)) "Undefined" 0 0))
  (bind _output_get (Variables|Default|SetMyWeapon _returnvalue))
  (Variables|/Script/Seven.Weapon|Setispossessed _output_get true)
  (CallFunction|AttachWeapon))

(fn SwitchWeapons
  (Utilities|FlowControl|ForLoopwithBreak 0 2 :!label _label
    (:LoopBody
      (Variables|Default|SetweaponToEquip%20Index (Math|Integer|%(Integer) (+ (Variables|Default|GetweaponToEquip%20Index) 1) 3))
      (Utilities|IsValid (.Icon (Utilities|Struct|BreakS_itemDetails (Utilities|Array|Get(acopy) (Variables|Default|GetRightHandItems) (Variables|Default|GetweaponToEquip%20Index))))
        (:Is%20Valid
          (Appearance|SetBrushfromTexture (Variables|/Game/Inventory_system/NewInventory/Inventory_widgets/Shortcut_Widget.Shortcut_Widget_C|GetR_weapons (Variables|Default|GetShortcutWidgetInstance)) (.Icon (Utilities|Struct|BreakS_itemDetails (Utilities|Array|Get(acopy) (Variables|Default|GetRightHandItems) (Variables|Default|GetweaponToEquip%20Index)))) false)
          (CallFunction|SpawnWeapon)
          (goto _label Break))
        (:Is%20Not%20Valid
          (Appearance|SetBrushfromTexture (Variables|/Game/Inventory_system/NewInventory/Inventory_widgets/Shortcut_Widget.Shortcut_Widget_C|GetR_weapons (Variables|Default|GetShortcutWidgetInstance)) 0 false))))))

(fn RemoveIconwhenUnequipped
  (params (Index :type Integer))
  (switch int Index
    (:0
      (Appearance|SetBrushfromTexture (Variables|/Game/Inventory_system/NewInventory/Inventory_widgets/WeaponsEquipSlot.WeaponsEquipSlot_C|GetweaponR1 (Variables|Default|GetweaponEquipSlotInstance)) 0 false))
    (:1
      (Appearance|SetBrushfromTexture (Variables|/Game/Inventory_system/NewInventory/Inventory_widgets/WeaponsEquipSlot.WeaponsEquipSlot_C|GetweaponR2 (Variables|Default|GetweaponEquipSlotInstance)) 0 false))
    (:2
      (Appearance|SetBrushfromTexture (Variables|/Game/Inventory_system/NewInventory/Inventory_widgets/WeaponsEquipSlot.WeaponsEquipSlot_C|GetweaponR3 (Variables|Default|GetweaponEquipSlotInstance)) 0 false))))

(fn SwitchItems
  (Utilities|FlowControl|ForLoopwithBreak 0 4 :!label _label
    (:LoopBody
      (bind _output_get (Variables|Default|SetitemToEquip (Math|Integer|%(Integer) (+ (Variables|Default|GetitemToEquip) 1) 5)))
      (Utilities|IsValid (.Icon (Utilities|Struct|BreakS_itemDetails (Utilities|Array|Get(acopy) (Variables|Default|GetLeftHandItems) _output_get)))
        (:Is%20Valid
          (Appearance|SetBrushfromTexture (Variables|/Game/Inventory_system/NewInventory/Inventory_widgets/Shortcut_Widget.Shortcut_Widget_C|GetL_weapons (Variables|Default|GetShortcutWidgetInstance)) (.Icon (Utilities|Struct|BreakS_itemDetails (Utilities|Array|Get(acopy) (Variables|Default|GetLeftHandItems) _output_get))) false)
          (goto _label Break))
        (:Is%20Not%20Valid
          (Appearance|SetBrushfromTexture (Variables|/Game/Inventory_system/NewInventory/Inventory_widgets/Shortcut_Widget.Shortcut_Widget_C|GetL_weapons (Variables|Default|GetShortcutWidgetInstance)) 0 false))))))

(fn CheckWhichItemtoUse
  (bind _lefthanditems (Variables|Default|GetLeftHandItems))
  (bind _itemtoequip (Variables|Default|GetitemToEquip))
  (bind _output (Utilities|Array|Get(acopy) _lefthanditems _itemtoequip))
  (bind _itemcount (Utilities|Struct|BreakS_itemDetails _output))
  (bind _returnvalue (- _itemcount 1))
  (if (< (Variables|Default|GetcurrentHealth) (Variables|Default|GetmaxHealth))
    (if (> _itemcount 0)
      (CallFunction|HealPlayer)
      (Utilities|Struct|SetmembersinS_itemDetails _output _returnvalue)
      (bind (_array_element _array_index) (Utilities|Array|ForEachLoopwithBreak (Variables|Default|GetInventoryItems) :!label _label)
        (:LoopBody
          (if (Utilities|Name|Equal(Name) (.itemname (Utilities|Array|Get(acopy) (Variables|Default|GetLeftHandItems) (Variables|Default|GetitemToEquip))) (.itemname _array_element))
            (Development|PrintString (Utilities|String|ToString(Integer) _array_index))
            (Utilities|Struct|SetmembersinS_itemDetails (Utilities|Array|Get(acopy) (Variables|Default|GetInventoryItems) _array_index) _returnvalue)
            (goto _label Break)))))))

(fn HealPlayer
  (Variables|Default|SetcurrentHealth (Math|Float|Clamp(Float) (+ (Variables|Default|GetcurrentHealth) (.usage (Utilities|Array|Get(acopy) (Variables|Default|GetLeftHandItems) (Variables|Default|GetitemToEquip)))) 0.0 (Variables|Default|GetmaxHealth))))