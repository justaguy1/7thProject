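; Treasure chest actor that the player opens with the Equip input to spawn a pickup.
; A box overlap with the player sets CanInteract on both chest and player and toggles the chest's input.
; GenerateItems spawns a PickUp_BP at the chest mesh location and plays the TreasureOpen animation.
; It then clears CanReOpen, so the chest yields only once.
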(event `self.ReceiveBeginPlay`
  (bind _asplayer_bp (cast `/Game/Blueprints/Player/Player_BP` (`GameplayStatics.GetPlayerCharacter` 0)))
  (set `self.Player` _asplayer_bp))

(event `self.Box.OnComponentBeginOverlap`
  (params (OverlappedComponent :type "PrimitiveComponent Object Reference") (OtherActor :type "Actor Object Reference") (OtherComp :type "PrimitiveComponent Object Reference") (OtherBodyIndex :type Integer) (bFromSweep :type Boolean) (SweepResult :type "HitResult Structure (by ref)"))
  (if (== OtherActor (`self.Player`))
    (set `/Game/Blueprints/Player/Player_BP.canInteract` true (`self.Player`))
    (set `self.canInteract` true)
    (`self.EnableInput` (`GameplayStatics.GetPlayerController` 0))))

(event `self.Box.OnComponentEndOverlap`
  (params (OverlappedComponent :type "PrimitiveComponent Object Reference") (OtherActor :type "Actor Object Reference") (OtherComp :type "PrimitiveComponent Object Reference") (OtherBodyIndex :type Integer))
  (if (== OtherActor (`self.Player`))
    (set `/Game/Blueprints/Player/Player_BP.canInteract` false (`self.Player`))
    (set `self.canInteract` false)
    (`self.DisableInput` (`GameplayStatics.GetPlayerController` 0))))

(event `InputAction|Equip`
  (params (Key :type "Key Structure"))
  (:`Pressed`
    (if (`self.canInteract`)
      (`self.GenerateItems`))))

(fn `GenerateItems`
  (if (`self.canReOpen`)
    (`|SpawnActorFromClass` "/Game/Widgets/NewInventory/Inventory_items/pickUp_BP.pickUp_BP_C" (`KismetMathLibrary.Conv_VectorToTransform` (`SceneComponent.K2_GetComponentLocation` (`self.Chesst`))) "Undefined" "OverrideRootScale" null null)
    (`SkeletalMeshComponent.PlayAnimation` (`self.Chesst`) "/Game/Meshes/StaticMesh/Treasure_Box/TreasureOpen.TreasureOpen" false)
    (set `self.canReOpen` false)))

(fn `UserConstructionScript`)