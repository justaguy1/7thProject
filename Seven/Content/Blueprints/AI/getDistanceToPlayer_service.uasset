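; Behavior tree service for enemy AI that tracks the distance between the controlled AI_BP pawn and the player.
; On each AI tick it measures the vector length to the player actor stored in the blackboard, then writes it to a distance key and the pawn's PlayerDistance.
; Without a valid player it writes a large fallback distance to the blackboard only.
; The SetWalkSpeed function is an empty stub.
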(event `self.ReceiveTickAI`
  (params (OwnerController :type "AIController Object Reference") (ControlledPawn :type "Pawn Object Reference") (DeltaSeconds :type "Float (single-precision)"))
  (bind _returnvalue (`BTFunctionLibrary.GetBlackboardValueAsActor` (`self.playerKeySelector`)))
  (bind _asenemy_aicontroller (cast `EnemyAIController` OwnerController))
  (bind _returnvalue_2 (`Controller.K2_GetPawn` _asenemy_aicontroller))
  (bind _asai_bp (cast `/Game/Blueprints/AI/AI_BP` _returnvalue_2))
  (set `self.ControlledPawn` _asai_bp)
  (`/Engine/EditorBlueprintResources/StandardMacros.IsValid` _returnvalue
    (:`Is Valid`
      (bind _returnvalue_3 (`KismetMathLibrary.VSize` (- (`Actor.K2_GetActorLocation` _returnvalue_2) (`Actor.K2_GetActorLocation` _returnvalue))))
      (`BTFunctionLibrary.SetBlackboardValueAsFloat` (`self.distanceKeySelector`) _returnvalue_3)
      (set `AIHumanCharacter.playerDistance` _returnvalue_3 (`self.ControlledPawn`)))
    (:`Is Not Valid`
      (`BTFunctionLibrary.SetBlackboardValueAsFloat` (`self.distanceKeySelector`) 5000.0))))

(fn `setWalkSpeed`)