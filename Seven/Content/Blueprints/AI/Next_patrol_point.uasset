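; Behavior tree task that advances an AI_BP pawn to the next patrol point in its PatrolLocation array.
; It writes the array entry at the blackboard index to the target key, then increments the index modulo the array length so patrols loop.
; It also prints a debug index one step beyond the newly stored one, then finishes with success.
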(event `self.ReceiveExecuteAI`
  (params (OwnerController :type "AIController Object Reference") (ControlledPawn :type "Pawn Object Reference"))
  (`self.incriment next patrol point` ControlledPawn)
  (`self.FinishExecute` true))

(fn `incriment next patrol point`
  (params (Object :type "Object Object Reference"))
  (locals (patrolPoints :type "Array of Actor Object Reference"))
  (bind _returnvalue (`BTFunctionLibrary.GetBlackboardValueAsInt` (`self.indexKey`)))
  (bind _returnvalue_2 (mod (+ _returnvalue 1) (`KismetArrayLibrary.Array_Length` (`local.patrolPoints`))))
  (bind _asai_bp (cast `/Game/Blueprints/AI/AI_BP` Object))
  (bind _output_get (set `local.patrolPoints` (`/Game/Blueprints/AI/AI_BP.patrol_Location` _asai_bp)))
  (`BTFunctionLibrary.SetBlackboardValueAsObject` (`self.TargetKey`) (`|GetArrayItem` _output_get _returnvalue))
  (`BTFunctionLibrary.SetBlackboardValueAsInt` (`self.indexKey`) _returnvalue_2)
  (`KismetSystemLibrary.PrintString` (`KismetStringLibrary.Conv_IntToString` _returnvalue_2))
  (return))