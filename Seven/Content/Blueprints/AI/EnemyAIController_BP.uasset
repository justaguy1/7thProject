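; Enemy AI controller that runs the AI_behaviour behavior tree and feeds it player information.
; On BeginPlay it starts the tree and stores the player character in the blackboard under a default actor key.
; When pawn sensing sees a Player_BP, it writes it to the visible actor key.
; Any sighting also copies the blackboard distance onto the controlled AI_BP and flags the player as in sight.
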(event `self.ReceiveBeginPlay`
  ;[1 1 1] Begin Play
  (`self.RunBehaviorTree` "/Game/Blueprints/AI/AI_behaviour.AI_behaviour")
  (bind _output_get (set `self.AIBlackboard` (`AIBlueprintHelperLibrary.GetBlackboard` (`self.K2_GetPawn`))))
  (`BlackboardComponent.SetValueAsObject` _output_get (`self.defaultActorKey`) (`GameplayStatics.GetPlayerCharacter` 0)))

(event `self.PawnSensing.OnSeePawn`
  (params (Pawn :type "Pawn Object Reference"))
  (`|ExecutionSequence`
    (:`then_1`
      (bind _asplayer_bp (cast `/Game/Blueprints/Player/Player_BP` Pawn))
      (`BlackboardComponent.SetValueAsObject` (`AIBlueprintHelperLibrary.GetBlackboard` (`self.K2_GetPawn`)) (`self.visible_actor_key`) _asplayer_bp))
    (:`then_2`
      (bind _asai_bp (cast `/Game/Blueprints/AI/AI_BP` (`self.K2_GetPawn`)))
      (`/Engine/EditorBlueprintResources/StandardMacros.IsValid` _asai_bp
        (:`Is Valid`
          (set `AIHumanCharacter.playerDistance` (`BlackboardComponent.GetValueAsFloat` (`self.AIBlackboard`) (`self.distanceKeyName`)) _asai_bp)
          (set `AIHumanCharacter.PlayerIsInSight` true _asai_bp))))))

(fn `UserConstructionScript`)