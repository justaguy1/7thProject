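; AI_BP is an enemy AI character that carries a weapon and shows a cone marker and health bar while targeted.
; BeginPlay sets montages, attaches a spawned weapon to the hand socket, creates the HUD and initializes patrol data.
; Tick mirrors anger to the Blackboard, smoothly turns toward the player when angry and montage-free, and switches walk speed on a montage flag.
; The patrol-target timeline is never run.
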(event `self.ReceiveBeginPlay`
  ;[1 1 1] Begin Play
  (`self.SetMontages`)
  (`SceneComponent.SetHiddenInGame` (`self.Cone`) true false)
  (set `self.Blackboard` (`AIBlueprintHelperLibrary.GetBlackboard` null))
  (bind _returnvalue (`|SpawnActorFromClass` "/Game/Blueprints/Weapons/Weapon_BP.Weapon_BP_C" (`KismetMathLibrary.MakeTransform` (0.0 0.0 0.0)) "Undefined" "OverrideRootScale" null null))
  (bind _output_get (set `self.MyWeapon` _returnvalue))
  (`self.K2_AttachToComponent` _output_get (`self.Mesh`) "WeaponRight" "SnapToTarget" "SnapToTarget" "KeepRelative" true)
  (set `Weapon.ispossessed` true (`self.MyWeapon`))
  (bind _returnvalue_2 (`|CreateWidget` "/Game/Blueprints/Huds/enemyHud.enemyHud_C" null self))
  (bind _output_get_2 (set `self.HealthBarHudinstance` _returnvalue_2))
  (`UserWidget.AddToViewport` _output_get_2 0)
  (set `self.patrolingDetail` (make `/Game/Blueprints/AI/PatrolStructure` false 0 (`KismetArrayLibrary.Array_Length` (`self.patrol_Location`)))))

(event `self.ReceiveTick`
  (params (DeltaSeconds :type "Float (single-precision)"))
  (`self.targetSystem`)
  (`BlackboardComponent.SetValueAsBool` (`self.Blackboard`) (`self.IsAgressiveKey`) (`self.isAngry`))
  (`self.rotateWhenAttacked`)
  (`self.disableMovementDuringAnimationMontage`))

(event `Key|LeftControl`
  (params (Key :type "Key Structure"))
  ;[1 1 1] walk / run
  (:`Pressed`
    (set `CharacterMovementComponent.MaxWalkSpeed` 600.0 (`self.CharacterMovement`)))
  (:`Released`
    (set `CharacterMovementComponent.MaxWalkSpeed` 300.0 (`self.CharacterMovement`))))

(fn `disableMovementDuringAnimationMontage`
  (if (`self.isMontageplaying`)
    (set `CharacterMovementComponent.MaxWalkSpeed` 300.0 (`self.CharacterMovement`))
    (else
      (set `CharacterMovementComponent.MaxWalkSpeed` 600.0 (`self.CharacterMovement`)))))

(fn `rotateWhenAttacked`
  (set `self.isMontageplaying` true)
  (if (and (`self.isAngry`) (not (`AnimInstance.IsAnyMontagePlaying` (`SkeletalMeshComponent.GetAnimInstance` (`self.Mesh`)))))
    (`/Engine/EditorBlueprintResources/StandardMacros.IsValid` (`GameplayStatics.GetPlayerCharacter` 0)
      (:`Is Valid`
        (`self.K2_SetActorRotation` (`KismetMathLibrary.RInterpTo` (`self.K2_GetActorRotation`) (`KismetMathLibrary.FindLookAtRotation` (`self.K2_GetActorLocation`) (`self.K2_GetActorLocation` (`GameplayStatics.GetPlayerCharacter` 0))) (`GameplayStatics.GetWorldDeltaSeconds`) 3.0))
        (set `self.isMontageplaying` false)))))

(fn `SetMontages`
  (set `self.animInstance` (`SkeletalMeshComponent.GetAnimInstance` (`self.Mesh`)))
  (set `self.attackMontage` (`|MakeArray` "/Game/Models/VampireAnimations/slash_01.slash_01" "/Game/Models/VampireAnimations/Attack_torch.Attack_torch" :!type "AnimMontage Object Reference"))
  (set `self.reactMontage` (`|MakeArray` "/Game/Models/VampireAnimations/react_left.react_left" "/Game/Models/VampireAnimations/react_right.react_right" :!type "AnimMontage Object Reference")))

(fn `targetSystem`
  (if (`self.targeted`)
    (`SceneComponent.SetHiddenInGame` (`self.Cone`) (not (`self.targeted`)) false)
    (set `self.canShowHealthBar` true)
    (`Widget.SetVisibility` (`self.HealthBarHudinstance`) "Visible")
    (else
      (`SceneComponent.SetHiddenInGame` (`self.Cone`) (not (`self.targeted`)) false)
      (set `self.canShowHealthBar` false)
      (`Widget.SetVisibility` (`self.HealthBarHudinstance`) "Hidden"))))

(fn `UserConstructionScript`)