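; comboAttack is an AI behavior tree task that appears to be an unfinished combo attack picker.
; On execute it validates the controlled pawn, casting it to AI_BP if invalid, then rolls a random index from five options, prints it and finishes successfully.
; A switch and a montage play call on the pawn's anim instance are left unconnected, so no attack animation plays.
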(event `self.ReceiveExecuteAI`
  (params (OwnerController :type "AIController Object Reference") (ControlledPawn :type "Pawn Object Reference"))
  (`/Engine/EditorBlueprintResources/StandardMacros.IsValid` (`self.controlledPawn`)
    (:`Is Valid`
      _)
    (:`Is Not Valid`
      (bind _asai_bp (cast `/Game/Blueprints/AI/AI_BP` ControlledPawn))
      (set `self.controlledPawn` _asai_bp)))
  (bind _output_get (set `self.count` (`KismetMathLibrary.RandomInteger` 5)))
  (`KismetSystemLibrary.PrintString` (`KismetStringLibrary.Conv_IntToString` _output_get))
  (`self.FinishExecute` true))