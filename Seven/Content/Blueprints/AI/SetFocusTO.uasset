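; Behavior tree task that sets or clears the AI controller's focus, switching on its SetFocus flag.
; When set, it focuses on the FocusKey blackboard actor and slows the AI_BP pawn's walk speed; otherwise it passes no focus actor and restores a faster speed.
; The pawn cast is cached and loops back to the validity check, with no failure exit, then the task finishes successfully.
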(event `self.ReceiveExecuteAI`
  (params (OwnerController :type "AIController Object Reference") (ControlledPawn :type "Pawn Object Reference"))
  (`/Engine/EditorBlueprintResources/StandardMacros.IsValid` (`self.ControlledAI`) :!label _label
    (:`Is Valid`
      (if (`self.setFocus?`)
        (`AIController.K2_SetFocus` OwnerController (`BTFunctionLibrary.GetBlackboardValueAsActor` (`self.focusKey`)))
        (set `CharacterMovementComponent.MaxWalkSpeed` 200.0 (`Character.CharacterMovement` (`self.ControlledAI`)))
        (else
          (`AIController.K2_SetFocus` OwnerController null)
          (set `CharacterMovementComponent.MaxWalkSpeed` 600.0 (`Character.CharacterMovement` (`self.ControlledAI`)))))
      (`self.FinishExecute` true))
    (:`Is Not Valid`
      (set `self.ControlledAI` (cast `/Game/Blueprints/AI/AI_BP` ControlledPawn :!pure true))
      (goto _label))))