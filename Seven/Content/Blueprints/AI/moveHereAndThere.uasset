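; Behavior Tree task that picks a strafe destination randomly to the left or right of the controlled AI pawn.
; It multiplies the stored distance by a random sign, then runs a debug-drawn Camera-channel trace along the pawn's right vector.
; A hit selects the full-distance point, while a miss selects the hit result's Location.
; The result is written to the AIMoveKey blackboard key and the task finishes successfully.
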(event `self.ReceiveExecuteAI`
  (params (OwnerController :type "AIController Object Reference") (ControlledPawn :type "Pawn Object Reference"))
  (bind _returnvalue (`Actor.K2_GetActorLocation` ControlledPawn))
  (bind _returnvalue_2 (+ _returnvalue (* (`Actor.GetActorRightVector` ControlledPawn) (`self.Distance_To_Starfe`))))
  (if (`KismetMathLibrary.RandomBool`)
    (set `self.starfeValue` 1.0)
    (else
      (set `self.starfeValue` -1.0)))
  (set `self.Distance_To_Starfe` (* (`self.Distance_To_Starfe`) (`self.starfeValue`)))
  (bind (_outhit _returnvalue_3) (`KismetSystemLibrary.LineTraceSingle` :`Start` _returnvalue :`End` _returnvalue_2 :`TraceChannel` "TraceTypeQuery2" :`DrawDebugType` "ForDuration"))
  (if _returnvalue_3
    (set `self.DIrection` _returnvalue_2)
    (else
      (set `self.DIrection` (`.Location` (`GameplayStatics.BreakHitResult` _outhit)))))
  (`BTFunctionLibrary.SetBlackboardValueAsVector` (`self.AI_moveKey`) (`self.DIrection`))
  (`self.FinishExecute` true))