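; Projectile actor that damages the player or AI characters when its sphere begins overlapping them.
; The sphere overlap checks whether the other actor is the player character and passes ProjectileDamage to ApplyProjectileDamage on Player_BP, guarded by a DoOnce.
; Any other actor is cast to AI_BP and damaged the same way, without the once-only guard.
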(event `self.Sphere.OnComponentBeginOverlap`
  (params (OverlappedComponent :type "PrimitiveComponent Object Reference") (OtherActor :type "Actor Object Reference") (OtherComp :type "PrimitiveComponent Object Reference") (OtherBodyIndex :type Integer) (bFromSweep :type Boolean) (SweepResult :type "HitResult Structure (by ref)"))
  (if (== OtherActor (`GameplayStatics.GetPlayerCharacter` 0))
    (bind _asplayer_bp (cast `/Game/Blueprints/Player/Player_BP` (`GameplayStatics.GetPlayerCharacter` 0)))
    (`/Engine/EditorBlueprintResources/StandardMacros.DoOnce` false
      (:`Completed`
        (`HumanCharacter.applyProjectileDamage` _asplayer_bp (`self.projectileDamage`))))
    (else
      (bind _asai_bp (cast `/Game/Blueprints/AI/AI_BP` OtherActor))
      (`HumanCharacter.applyProjectileDamage` _asai_bp (`self.projectileDamage`)))))

(fn `UserConstructionScript`)